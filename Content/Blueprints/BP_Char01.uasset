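; Player-controlled pawn with camera look, walking and an E-key door interaction.
; Axis input adds movement scaled by MaxSpeed along the actor's forward and right vectors, which Tick consumes and applies as an unswept, delta-time-scaled local offset.
; Pressing E runs a debug-drawn WorldStatic line trace from the camera, calls OpenDoorMessage on the hit actor and adds the returned rotation to that actor's local rotation.
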(event EventBeginPlay)

(event Collision|EventActorBeginOverlap
  (params (OtherActor :type Actor%20Object%20Reference)))

(event EventTick
  (params (DeltaSeconds :type Float%20%28single-precision%29))
  (bind _returnvalue (Class|Pawn|ConsumeMovementInputVector))
  (Transformation|AddActorLocalOffset (* _returnvalue DeltaSeconds) false false))

(event Input|AxisEvents|InputAxisMoveForward
  (params (AxisValue :type Float%20%28single-precision%29))
  (Pawn|Input|AddMovementInput (Transformation|GetActorForwardVector) (* AxisValue (Variables|Default|GetMaxSpeed)) false))

(event Input|AxisEvents|InputAxisMoveRight
  (params (AxisValue :type Float%20%28single-precision%29))
  (Pawn|Input|AddMovementInput (Transformation|GetActorRightVector) (* AxisValue (Variables|Default|GetMaxSpeed)) false))

(event Input|AxisEvents|InputAxisLookUp
  (params (AxisValue :type Float%20%28single-precision%29))
  (Pawn|Input|AddControllerPitchInput AxisValue))

(event Input|AxisEvents|InputAxisTurn
  (params (AxisValue :type Float%20%28single-precision%29))
  (Pawn|Input|AddControllerYawInput AxisValue))

(event Input|KeyboardEvents|E
  (params (Key :type Key%20Structure :default "None"))
  (bind _camera (Variables|Camera|GetCamera))
  (bind _returnvalue (Transformation|GetWorldLocation _camera))
  (:Pressed
    (bind _outhit (Collision|LineTraceForObjects _returnvalue (+ _returnvalue (* (Math|Vector|GetForwardVector _camera) 500)) (Utilities|Array|MakeArray "ObjectTypeQuery1") false 0 "ForDuration" true "(R=1.000000,G=0.000000,B=0.000000,A=1.000000)" "(R=0.000000,G=1.000000,B=0.000000,A=1.000000)" 2e+01))
    (bind _openvalue (Class|BPCharInterface|OpenDoor(Message) (.HitActor (Collision|BreakHitResult _outhit))))
    (Transformation|AddActorLocalRotation (.HitActor (Collision|BreakHitResult _outhit)) _openvalue false false)))

(fn ConstructionScript)