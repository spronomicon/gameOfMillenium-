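; BP_InteractiveFromTriger is a trigger volume that activates or deactivates a linked interactive actor through message calls.
; Box begin and end overlap send Activate and Deactivate messages to ActorToInteractiove, without filtering the overlapping actor, and print the returned result.
; It also has its own Activate and Deactivate functions, which print debug text, toggle Opened and return true.
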(event OnComponentBeginOverlap(Box)
  (params (OverlappedComponent :type Primitive%20Component%20Object%20Reference) (OtherActor :type Actor%20Object%20Reference) (OtherComp :type Primitive%20Component%20Object%20Reference) (OtherBodyIndex :type Integer) (bFromSweep :type Boolean) (SweepResult :type Hit%20Result%20Structure%20%28by%20ref%29))
  (bind _succsess (Class|BPIInteraction|Activate(Message) (Variables|Default|GetActor%20to%20Interactiove)))
  (if _succsess
    (Development|PrintString "Activate True")
    (else
      (Development|PrintString "Activate False"))))

(event OnComponentEndOverlap(Box)
  (params (OverlappedComponent :type Primitive%20Component%20Object%20Reference) (OtherActor :type Actor%20Object%20Reference) (OtherComp :type Primitive%20Component%20Object%20Reference) (OtherBodyIndex :type Integer))
  (bind _succsess (Class|BPIInteraction|Deactivate(Message) (Variables|Default|GetActor%20to%20Interactiove)))
  (if _succsess
    (Development|PrintString "Deactivate True")
    (else
      (Development|PrintString "Deactivate False"))))

(event EventBeginPlay)

(event EventTick
  (params (DeltaSeconds :type Float%20%28single-precision%29)))

(fn ConstructionScript)

(fn Activate
  (Development|PrintString "Activate Function Worked")
  (Variables|Default|SetOpened true)
  (return true))

(fn Deactivate
  (Development|PrintString "Deactivate Function Worked")
  (Variables|Default|SetOpened false)
  (return true))